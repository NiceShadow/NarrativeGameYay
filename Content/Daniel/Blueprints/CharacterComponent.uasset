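; Character component that triggers the matching dialogue whenever an interactable object is selected, across what appear to be several puzzle rooms.
; The Interact event switches on a Selection value for furniture, props and doors, calling that object's dedicated function on the dialogue window.
; GetDialogueW fetches that window from BP_OurHUD through the first player controller on each call.
; The component holds no dialogue or puzzle logic itself, only the routing.
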(event Custom|Interact
  (params (Selection :type String))
  (bind _newparam (CallFunction|GetDialogueW))
  (bind _newparam_2 (CallFunction|GetDialogueW))
  (bind _newparam_3 (CallFunction|GetDialogueW))
  (bind _newparam_4 (CallFunction|GetDialogueW))
  (switch string Selection
    (:tv
      (Default|InteractTV _newparam_3))
    (:shelf
      (Default|InteractShelf _newparam_3))
    (:mirror
      (Default|InteractMirror _newparam_3))
    (:bed
      (Default|InteractBed _newparam_3))
    (:couch
      (Default|InteractCouch _newparam_3))
    (:notepad
      (Default|NotepadFound _newparam_3))
    (:safe
      (Default|InteractSafe _newparam_3))
    (:carpet
      (Default|InteractCarpet _newparam_3))
    (:phone
      (Default|InteractPhone _newparam_3))
    (:bdoor
      (Default|InteractBdoor _newparam_3))
    (:door
      (Default|InteractDoor _newparam_3))
    (:chute
      (Default|InteractLaundryChute _newparam_3))
    (:dials
      (Default|InteractLeftDesk _newparam_3))
    (:sharpener
      (Default|InteractRightDesk _newparam_3))
    (:window
      (Default|InteractWindow _newparam_3))
    (:nail
      (Default|InteractPlant _newparam_3))
    (:wmachine
      (Default|InteractWmachine _newparam))
    (:kdoor
      (Default|Room2Door _newparam))
    (:wmachine1
      (Default|Room2Wmachine1 _newparam))
    (:wmachine2
      (Default|Room2Wmachine2 _newparam))
    (:wmachine3
      (Default|Room2Wmachine3 _newparam))
    (:dryer1
      (Default|Room2DryerEmpty _newparam :!label _label))
    (:dryer2
      (goto _label))
    (:dryer3
      (Default|Room2DryerTooS _newparam))
    (:wm2_wetclothes
      (Default|InteractwithWetClothes _newparam))
    (:closet
      (Default|Room2OpenCloset _newparam))
    (:waterstain
      (Default|InteractWaterstain _newparam))
    (:towel
      (Default|Room2LaundryBasket _newparam))
    (:dirtyclothes
      (Default|Room2DirtyClothes _newparam))
    (:mixer
      (Default|Room3Mixer _newparam_2))
    (:shelf1
      (Default|Room3Shelf1 _newparam_2))
    (:shelf2
      (Default|Room3Shelf2 _newparam_2))
    (:shelf3
      (Default|Room3Shelf3 _newparam_2))
    (:waterstain1
      (Default|Room3Waterstain _newparam_2))
    (:pot
      (Default|Room3Pot _newparam_2))
    (:island
      (Default|Room3KitchenIsland _newparam_2))
    (:flour
      (Default|Room3Flour _newparam_2))
    (:cable
      (Default|Room3Cable _newparam_2))
    (:backdoor
      (Default|Room3Backdoor _newparam_2))
    (:fridge
      (Default|Fridge _newparam_4))
    (:toilet
      (Default|Toilet _newparam_4))))

(fn GetDialogueW
  (bind _asbp_our_hud (Utilities|Casting|CastToBP_OurHUD (HUD|GetHUD (Game|GetPlayerController 0))))
  (return (Variables|/Game/Blueprints/BP_OurHUD.BP_OurHUD_C|GetDialogueWindow _asbp_our_hud)))