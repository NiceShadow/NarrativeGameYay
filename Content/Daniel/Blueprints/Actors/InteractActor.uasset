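; InteractActor is an actor Blueprint that takes one of two component forms, chosen by its Sphere flag.
; Its construction script destroys the Box component when Sphere is true and the Cylinder component otherwise, leaving only one in place.
; Unconnected leftover nodes that toggle visibility and collision never run, and the file shows no interaction logic.
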(fn ConstructionScript
  (if (Variables|Default|GetSphere?)
    (Components|DestroyComponent (Variables|Default|GetBox))
    (else
      (Components|DestroyComponent (Variables|Default|GetCylinder)))))