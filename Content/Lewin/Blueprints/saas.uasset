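; Pop-up book actor for room 1 of an adventure game, unfolding through skeletal animations and hosting the room's puzzle interactions.
; Events animate or swap materials for props like the door, safe, bed, painting and laundry chute, setting progress flags; gum plus tape fixes the cable.
; The TV plays media channels with timed shutoff.
; InteractActors, grouped by tag, toggle collision as the player enters the bathroom and are destroyed once used.
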(event Custom|Open
  ;[1 1 1] Open gerneral
  (Variables|Default|SetCustomTimeDilation 0.605)
  (Components|Animation|PlayAnimation (Variables|Default|Getbook) "/Game/Jana/bookwUV/bookUV_17_Anim.bookUV_17_Anim" false)
  ;;[0 0 0] Room1
  (Components|Animation|PlayAnimation (Variables|Default|Get01_safe_lewin) "/Game/Lewin/01_Room/animations/01_safe_open.01_safe_open" false)
  (Components|Animation|PlayAnimation (Variables|Default|Get01_added_lewin) "/Game/Lewin/01_Room/animations/addedelements_frozenplantsX_Popupbasic.addedelements_frozenplantsX_Popupbasic" false)
  (Components|Animation|PlayAnimation (Variables|Default|Get01_unsafe_lewin) "/Game/Lewin/01_Room/animations/01_unsafe_open.01_unsafe_open" false)
  (Utilities|FlowControl|Delay 0.15)
  (Development|SetHiddeninGame (Variables|Default|GetcarpetTV_Scene) false true)
  ;[1 1 1] Test run different events
  (Rendering|Material|SetMaterial (Variables|Default|Get01_unsafe_lewin) 5 "/Game/Materials/Assets/Room1/Textures/M_r1_bathroom_wall.M_r1_bathroom_wall")
  (Development|SetHiddeninGame (Variables|Default|GetcableGUM) true false))

(event Custom|SetRightWallTransparent
  (params (yes :type Boolean))
  (bind _returnvalue (Game|GetPlayerCharacter 0))
  (bind _plane3 (Variables|Default|GetPlane3))
  ;[1 1 1] Set right wall transparent
  (if yes
    (Rendering|Material|SetMaterial (Variables|Default|Get01_safe_lewin) 1 "/Game/Materials/Assets/Room1/Textures/RightWallAlpha.RightWallAlpha")
    (Rendering|Material|SetMaterial (Variables|Default|GetRightWallDoor) 0 "/Game/Materials/Assets/Room1/Textures/RightDoorAlpha.RightDoorAlpha")
    (bind _asmain_character (Utilities|Casting|CastToMainCharacter _returnvalue))
    (Variables|/Game/Lewin/Blueprints/MainCharacter.MainCharacter_C|Setr1_rightwallTransparent _asmain_character true)
    (Rendering|Material|SetMaterial _plane3 0 "/Game/Lewin/video/ingame/M_TVMedia_Trans.M_TVMedia_Trans")
    (else
      (Rendering|Material|SetMaterial (Variables|Default|Get01_safe_lewin) 1 "/Game/Materials/Assets/Room1/Textures/M_r1_right_wall.M_r1_right_wall")
      (Rendering|Material|SetMaterial (Variables|Default|GetRightWallDoor) 0 "/Game/Materials/Assets/Room1/Textures/M_r1_door_right_wall.M_r1_door_right_wall")
      (bind _asmain_character_2 (Utilities|Casting|CastToMainCharacter _returnvalue))
      (Variables|/Game/Lewin/Blueprints/MainCharacter.MainCharacter_C|Setr1_rightwallTransparent _asmain_character_2 false)
      (Rendering|Material|SetMaterial _plane3 0 "/Game/Lewin/video/ingame/LoveMP_Video_Mat.LoveMP_Video_Mat"))))

(event Custom|StartLightFlickering)

(event Custom|MoveCarpetAway
  (CallFunction|MyPlaySound "/Game/Sounds/SFX/00_-_sfx_-_s_r1_011_shoving_carpet.00_-_sfx_-_s_r1_011_shoving_carpet")
  (Variables|Default|Setr1_carpetTVmoved true)
  (bind _newtrack_0 (Timeline|Timeline_4 PlayFromStart)
    (:Update
      (Transformation|SetRelativeLocation (Variables|Default|GetcarpetTV_Scene) (Math|Vector|MakeVector (Math|Float|Lerp 3.8 3.0 _newtrack_0) (Math|Float|Lerp 0.0 -3.8 _newtrack_0) 0.0) false false)
      (Transformation|SetRelativeRotation (Variables|Default|GetcarpetTV_Scene) (Math|Rotator|MakeRotator 0.0 0.0 (Math|Float|Lerp 0.0 25.0 _newtrack_0)) false false))))

(event Custom|GumOnCable
  (CallFunction|MyPlaySound "/Game/Sounds/SFX/00_-_sfx_-_s_r1_013_gum_fixing.00_-_sfx_-_s_r1_013_gum_fixing")
  (Variables|Default|Setr1_gumPutOnCable true)
  (Development|SetHiddeninGame (Variables|Default|GetcableGUM) false false)
  (if (Variables|Default|Getr1_tapePutOnCable)
    (Development|SetHiddeninGame (Variables|Default|GetcableFix) false false)
    (Default|2ndFix (Variables|/Game/Blueprints/BP_OurPC.BP_OurPC_C|GetDiaRef (Variables|Default|GetPC_Ref)))
    (CallFunction|RemoveActorInterbyTag "carpet")
    (Variables|Default|Setr1_cableFixed true)
    (else
      (Default|1stFix (Variables|/Game/Blueprints/BP_OurPC.BP_OurPC_C|GetDiaRef (Variables|Default|GetPC_Ref))))))

(event Custom|TapeOnCable
  (CallFunction|MyPlaySound "/Game/Sounds/SFX/00_-_sfx_-_s_r1_014_tape_fixing.00_-_sfx_-_s_r1_014_tape_fixing")
  (Variables|Default|Setr1_tapePutOnCable true)
  (Development|SetHiddeninGame (Variables|Default|GetcableTape) false false)
  (if (Variables|Default|Getr1_gumPutOnCable)
    (Development|SetHiddeninGame (Variables|Default|GetcableFix) false false)
    (Default|2ndFix (Variables|/Game/Blueprints/BP_OurPC.BP_OurPC_C|GetDiaRef (Variables|Default|GetPC_Ref)))
    (CallFunction|RemoveActorInterbyTag "carpet")
    (Variables|Default|Setr1_cableFixed true)
    (else
      (Default|1stFix (Variables|/Game/Blueprints/BP_OurPC.BP_OurPC_C|GetDiaRef (Variables|Default|GetPC_Ref))))))

(event Custom|TurnTVOffAfterTime
  (params (Time :type Float%20%28single-precision%29))
  (Utilities|Time|ClearandInvalidateTimerbyHandle (Variables|Default|GetTVTimer))
  (bind _returnvalue (Utilities|Time|SetTimerbyEvent (delegate Custom|TurnOfTVafterTimer) Time))
  (Variables|Default|SetTVTimer _returnvalue))

(event Custom|TurnOfTVafterTimer
  (CallFunction|PlayTV -1))

(event Custom|Hop%20in%20laundry%20chute
  (Variables|Default|SetCharacterLocationBeforeHopping (Transformation|GetActorLocation (Game|GetPlayerCharacter 0)))
  (bind _newtrack_0 (Timeline|Timeline_5 PlayFromStart)
    (:Update
      (Transformation|SetActorLocation (Game|GetPlayerCharacter 0) (Math|Vector|MakeVector (.X (Math|Vector|BreakVector (Math|Vector|Lerp(Vector) (Variables|Default|GetCharacterLocationBeforeHopping) (Transformation|GetWorldLocation (Variables|Default|GetLaundryHoppingCharLoc)) _newtrack_0))) (.Y (Math|Vector|BreakVector (Math|Vector|Lerp(Vector) (Variables|Default|GetCharacterLocationBeforeHopping) (Transformation|GetWorldLocation (Variables|Default|GetLaundryHoppingCharLoc)) _newtrack_0))) (.Z (Math|Vector|BreakVector (Transformation|GetActorLocation (Game|GetPlayerCharacter 0))))) false false))
    (:Finished
      (bind _asmain_character (Utilities|Casting|CastToMainCharacter (Game|GetPlayerCharacter 0)))
      (Default|HopinLaundry _asmain_character)
      (Utilities|FlowControl|Delay 1.0)
      (CallFunction|MyPlaySound "/Game/Sounds/SFX/00_-_sfx_-_s_r1_021_laundry_chute_sliding.00_-_sfx_-_s_r1_021_laundry_chute_sliding"))))

(event Custom|OpenPhoneInterface
  (Default|ShowInterface (Variables|/Game/Lewin/UI/WB_GameUI.WB_GameUI_C|GetPhoneInterface (Variables|/Game/Blueprints/BP_OurPC.BP_OurPC_C|GetGameUIRef (Variables|Default|GetPC_Ref))) true)
  (Default|StartUsingPhone (CallFunction|GetCharRef)))

(event Custom|CableElectoShockParticle
  (Effects|SpawnEmitteratLocation "/Game/StarterContent/Particles/P_ElectroShock.P_ElectroShock" (Transformation|GetWorldLocation (Variables|Default|GetcableGUM))))

(event Custom|RandStuff
  ;[1 1 1] Test run different events
  (Utilities|FlowControl|MultiGate false false 0
    (:Out%201
      (CallFunction|MoveCarpetAway))
    (:Out%202
      (CallFunction|GumonCable))
    (:Out%203
      (CallFunction|TapeonCable))
    (:Out%204
      (CallFunction|MessUpBed))
    (:Out%205
      (CallFunction|OpenDoor1))
    (:Out%206
      (CallFunction|OpenLaundryChute))
    (:Out%207
      (CallFunction|PaintingFall))
    (:Out%208
      (CallFunction|OpenSafe))
    (:Out%209
      (CallFunction|PlayTV))
    (:Out%2010
      (CallFunction|PlayTV 1))
    (:Out%2011
      (CallFunction|PlayTV 2))))

(event Custom|HideNotepad
  (Rendering|Material|SetMaterial (Variables|Default|Get01_added_lewin) 8 "/Game/Materials/M_Transparent.M_Transparent"))

(event Custom|StartPhone
  (params (in :type Boolean))
  (bind _phoneradius (Variables|Default|GetphoneRadius))
  (Rendering|Material|SetMaterial (Variables|Default|Get01_added_lewin) 12 (select in "/Game/Materials/Assets/Room1/Textures/M_phonebody.M_phonebody" "/Game/Materials/Assets/Room1/Textures/M_phone.M_phone"))
  (if in
    (CallFunction|MyPlaySound "/Game/Sounds/SFX/00_-_sfx_-_s_r1_015_phone_pick_up.00_-_sfx_-_s_r1_015_phone_pick_up")
    (Collision|SetCollisionEnabled _phoneradius "QueryAndPhysics")
    (else
      (CallFunction|MyPlaySound "/Game/Sounds/SFX/00_-_sfx_-_s_r1_016_phone_hang_up.00_-_sfx_-_s_r1_016_phone_hang_up")
      (Collision|SetCollisionEnabled _phoneradius "NoCollision"))))

(event Custom|InBathroom
  (params (characterIsInBathroom :type Boolean))
  (bind _output_get (Variables|Default|SetcharacterIsInBathroom characterIsInBathroom))
  (if _output_get
    (CallFunction|ChangeCollisionOfInteractActors false (Variables|Default|GetInteractablesIF_RightWall))
    (CallFunction|ChangeCollisionOfInteractActors true (Variables|Default|GetInteractablesBehind_RightWall))
    (else
      (CallFunction|ChangeCollisionOfInteractActors true (Variables|Default|GetInteractablesIF_RightWall))
      (CallFunction|ChangeCollisionOfInteractActors false (Variables|Default|GetInteractablesBehind_RightWall)))))

(event Custom|StopTVInstant
  (if (Utilities|Time|IsValidTimerHandle (Variables|Default|GetTVTimer))
    (CallFunction|PlayTV -1)
    (Development|PrintString "sssssssssssssssss")))

(event Custom|PickUpNotepad
  (CallFunction|RemoveActorInterbyTag "notepad"))

(event Custom|OpenSafeInterface
  ;[1 1 1] Test run different events
  (Default|ShowInterface (Variables|/Game/Lewin/UI/WB_GameUI.WB_GameUI_C|GetSafeInterface (Variables|/Game/Blueprints/BP_OurPC.BP_OurPC_C|GetGameUIRef (Variables|Default|GetPC_Ref))) true))

(event Custom|OpenLaundryChute
  ;[1 1 1] OpenLaundryChute
  (Variables|Default|Setr1_LaundryChuteOpened true)
  (bind _newtrack_0 (Timeline|Timeline_0 PlayFromStart)
    (:Update
      (Transformation|SetRelativeRotation (Variables|Default|GetLaundryDoorAxis) (Math|Rotator|MakeRotator 0.0 (Math|Float|Lerp 0.0 1.1e+02 _newtrack_0) 0.0) false false))))

(event Custom|OpenSafe
  ;[1 1 1] OpenSafe
  (Variables|Default|Setr1_SafeOpened true)
  (bind _newtrack_0 (Timeline|Timeline_2 PlayFromStart)
    (:Update
      (Transformation|SetRelativeRotation (Variables|Default|GetSafeRot) (Math|Rotator|MakeRotator 0.0 0.0 (Math|Float|Lerp 0.0 -3e+01 _newtrack_0)) false false))))

(event Custom|PaintingFall
  ;[1 1 1] Painting Falling
  (Utilities|FlowControl|Sequence
    (:then_0
      (Variables|Default|Setr1_PaintingFallenDown true)
      (Components|Animation|PlayAnimation (Variables|Default|Get01_added_lewin) "/Game/Lewin/01_Room/animations/addedelements_frozenplantsX_pfalling__1_.addedelements_frozenplantsX_pfalling__1_" false)
      (Utilities|FlowControl|Delay (/ (CallFunction|RealtoCustomTime 1.83) 1.2))
      (Collision|SetCollisionEnabled (Variables|Default|GetpaintingBox) "QueryAndPhysics"))
    (:then_1
      (Utilities|FlowControl|Delay 0.1)
      (CallFunction|MyPlaySound "/Game/Sounds/SFX/PaintingFallTest.PaintingFallTest")
      (Utilities|FlowControl|Delay 0.4)
      (CallFunction|MyPlaySound "/Game/Sounds/SFX/PaintingFallTest.PaintingFallTest")
      (Utilities|FlowControl|Delay 0.5)
      (CallFunction|MyPlaySound "/Game/Sounds/SFX/PaintingFallTest.PaintingFallTest")
      (Utilities|FlowControl|Delay 0.3)
      (CallFunction|MyPlaySound "/Game/Sounds/SFX/PaintingFallTest.PaintingFallTest")
      (Utilities|FlowControl|Delay 0.6)
      (CallFunction|MyPlaySound "/Game/Sounds/SFX/PaintingFallTest.PaintingFallTest"))))

(event Custom|PlayTV
  (params (channel :type Integer))
  ;[1 1 1] TV
  (bind _output_get (Variables|Default|SetCurrentTVChannel channel))
  (switch int _output_get
    (:-1
      (Rendering|SetVisibility (Variables|Default|GetPlane3) false true)
      (Media|MediaPlayer|Close (Variables|Default|GetLoveMT) :!class /Script/MediaAssets.MediaPlayer)
      (Utilities|Time|ClearandInvalidateTimerbyHandle (Variables|Default|GetTVTimer)))
    (:0
      (Class|MediaPlayer|OpenSourceLatent (Variables|Default|GetLoveMT) "/Game/Lewin/video/ingame/snowTV.snowTV" (Utilities|Struct|MakeMediaPlayerOptions "(Audio=0,Caption=-1,Metadata=-1,Script=-1,Subtitle=-1,Text=-1,Video=0)" "+00000000.00:00:00.000000000" "UseMediaPlayerSetting" "UseMediaPlayerSetting"))
      (Utilities|FlowControl|Delay 0.1)
      (Rendering|SetVisibility (Variables|Default|GetPlane3) true true)
      (Rendering|Material|SetMaterial (Variables|Default|GetPlane4) 0 "/Game/Lewin/video/ingame/SnowGlowMaterial.SnowGlowMaterial")
      (CallFunction|TurnTVOffAfterTime 7.9))
    (:1
      (Class|MediaPlayer|OpenSourceLatent (Variables|Default|GetLoveMT) "/Game/Lewin/video/ingame/loveTVscene.loveTVscene" (Utilities|Struct|MakeMediaPlayerOptions "(Audio=0,Caption=-1,Metadata=-1,Script=-1,Subtitle=-1,Text=-1,Video=0)" "+00000000.00:00:00.000000000" "UseMediaPlayerSetting" "UseMediaPlayerSetting"))
      (Utilities|FlowControl|Delay 0.1)
      (Rendering|SetVisibility (Variables|Default|GetPlane3) true true)
      (Rendering|Material|SetMaterial (Variables|Default|GetPlane4) 0 "/Game/Lewin/video/ingame/LoveGlowMat.LoveGlowMat")
      (CallFunction|TurnTVOffAfterTime 15.0))
    (:2
      (Class|MediaPlayer|OpenSourceLatent (Variables|Default|GetLoveMT) "/Game/Lewin/video/ingame/tvnews3.tvnews3" (Utilities|Struct|MakeMediaPlayerOptions "(Audio=0,Caption=-1,Metadata=-1,Script=-1,Subtitle=-1,Text=-1,Video=0)" "+00000000.00:00:00.000000000" "UseMediaPlayerSetting" "UseMediaPlayerSetting"))
      (Utilities|FlowControl|Delay 0.1)
      (Rendering|SetVisibility (Variables|Default|GetPlane3) true true)
      (Media|MediaPlayer|OpenSource (Variables|Default|GetLoveGlow) "/Game/Lewin/video/ingame/newsGlow.newsGlow")
      (Rendering|Material|SetMaterial (Variables|Default|GetPlane4) 0 "/Game/Lewin/video/ingame/TVGlow.TVGlow")
      (CallFunction|TurnTVOffAfterTime 41.099998))))

(event Custom|OpenDoor1
  ;[1 1 1] Open Door
  (CallFunction|RemoveActorInterbyTag "bdoor")
  (CallFunction|MyPlaySound "/Game/Sounds/SFX/00_-_sfx_-_s_r1_020_pressing_down_handle.00_-_sfx_-_s_r1_020_pressing_down_handle")
  (Variables|Default|Setr1_doorOpened true)
  (Components|Animation|PlayAnimation (Variables|Default|Get01_unsafe_lewin) "/Game/Lewin/01_Room/animations/01_UNsafeelement_bropening.01_UNsafeelement_bropening" false)
  (bind _newtrack_0 (Timeline|Timeline_1 PlayFromStart)
    (:Update
      (Transformation|SetRelativeRotation (Variables|Default|GetDoorRot) (Math|Rotator|MakeRotator 0.0 0.0 (Math|Float|Lerp 0.0 1e+02 _newtrack_0)) false false))))

(event Custom|MessUpBed
  ;[1 1 1] MessUpBed
  (Variables|Default|Setr1_BedMessedUp true)
  (Rendering|Material|SetMaterial (Variables|Default|Get01_safe_lewin) 8 "/Game/Materials/Assets/Room1/Textures/M_r1_messed_up_bed_rear.M_r1_messed_up_bed_rear")
  (Rendering|Material|SetMaterial (Variables|Default|Get01_safe_lewin) 7 "/Game/Materials/Assets/Room1/Textures/M_r1_messed_up_bed_top.M_r1_messed_up_bed_top")
  (CallFunction|RemoveActorInterbyTag "bed"))

(event EventBeginPlay
  (Development|SetHiddeninGame (Variables|Default|GetLaundryHoppingCharLoc) true true)
  (Development|SetHiddeninGame (Variables|Default|GetPlane2) true true)
  (Collision|SetActorEnableCollision false)
  (CallFunction|StartLightFlickering)
  (bind _asbp_our_pc (Utilities|Casting|CastToBP_OurPC (Game|GetPlayerController 0)))
  (Variables|Default|SetPC_Ref _asbp_our_pc)
  (Development|SetHiddeninGame (Variables|Default|GetCables) true true)
  (Rendering|Material|SetMaterial (Variables|Default|Get01_unsafe_lewin) 5 "/Game/Materials/M_Transparent.M_Transparent")
  (CallFunction|GetInteractActors)
  (CallFunction|ChangeCollisionOfInteractActors false (Variables|Default|GetInteractablesBehind_RightWall)))

(fn ConstructionScript
  (if (Variables|Default|Getdev)
    (Variables|/Script/Engine.SkeletalMeshComponent|SetAnimationData (Variables|Default|Getbook) (Utilities|Struct|MakeSingleAnimationPlayData "/Game/Jana/bookwUV/bookUV_17_Anim.bookUV_17_Anim" true false 2.0))
    (Variables|/Script/Engine.SkeletalMeshComponent|SetAnimationData (Variables|Default|Get01_safe_lewin) (Utilities|Struct|MakeSingleAnimationPlayData "/Game/Lewin/01_Room/animations/01_safe_open.01_safe_open" true false 2.0))
    (Variables|/Script/Engine.SkeletalMeshComponent|SetAnimationData (Variables|Default|Get01_added_lewin) (Utilities|Struct|MakeSingleAnimationPlayData "/Game/Lewin/01_Room/animations/addedelements_frozenplantsX_Popupbasic.addedelements_frozenplantsX_Popupbasic" true false 2.0))
    (Variables|/Script/Engine.SkeletalMeshComponent|SetAnimationData (Variables|Default|Get01_unsafe_lewin) (Utilities|Struct|MakeSingleAnimationPlayData "/Game/Lewin/01_Room/animations/01_unsafe_open.01_unsafe_open" true false 2.0))
    (else
      (Variables|/Script/Engine.SkeletalMeshComponent|SetAnimationData (Variables|Default|Getbook) (Utilities|Struct|MakeSingleAnimationPlayData "/Game/Jana/bookwUV/bookUV_17_Anim.bookUV_17_Anim" true false 0.0))
      (Variables|/Script/Engine.SkeletalMeshComponent|SetAnimationData (Variables|Default|Get01_safe_lewin) (Utilities|Struct|MakeSingleAnimationPlayData "/Game/Lewin/01_Room/animations/01_safe_open.01_safe_open" true false 0.0))
      (Variables|/Script/Engine.SkeletalMeshComponent|SetAnimationData (Variables|Default|Get01_added_lewin) (Utilities|Struct|MakeSingleAnimationPlayData "/Game/Lewin/01_Room/animations/addedelements_frozenplantsX_Popupbasic.addedelements_frozenplantsX_Popupbasic" true false 0.0))
      (Variables|/Script/Engine.SkeletalMeshComponent|SetAnimationData (Variables|Default|Get01_unsafe_lewin) (Utilities|Struct|MakeSingleAnimationPlayData "/Game/Lewin/01_Room/animations/01_unsafe_open.01_unsafe_open" true false 0.0)))))

(fn RealtoCustomTime
  (params (real :type Float%20%28single-precision%29))
  (return (/ real (Variables|Default|GetCustomTimeDilation))))

(fn MyPlaySound
  (params (Sound :type Sound%20Base%20Object%20Reference))
  (Audio|PlaySound2D Sound (Variables|/Game/Blueprints/BP_OurPC.BP_OurPC_C|GetSoundEffectsVolume (Variables|Default|GetPC_ref)) 1.0 0.0 0 0))

(fn GetCharRef
  (bind _asmain_character (Utilities|Casting|CastToMainCharacter (Game|GetPlayerCharacter 0)))
  (return _asmain_character))

(fn GetInteractActors
  (Utilities|Array|Clear (Variables|Default|GetInteractablesIF_RightWall))
  (Utilities|Array|Clear (Variables|Default|GetInteractablesBehind_RightWall))
  (bind _outactors (Actor|GetAllActorsOfClass "/Game/Daniel/Blueprints/Actors/InteractActor.InteractActor_C"))
  (for _array_element _outactors
    (if (Math|Boolean|ORBoolean (Utilities|Name|Equal(Name) (Utilities|Array|Get(acopy) (Variables|/Script/Engine.Actor|GetTags _array_element) 1) "shelf") (Utilities|Name|Equal(Name) (Utilities|Array|Get(acopy) (Variables|/Script/Engine.Actor|GetTags _array_element) 1) "mirror") (Utilities|Name|Equal(Name) (Utilities|Array|Get(acopy) (Variables|/Script/Engine.Actor|GetTags _array_element) 1) "chute"))
      (Utilities|Array|Add (Variables|Default|GetInteractablesBehind_RightWall) _array_element)
      (else
        (Utilities|Array|Add (Variables|Default|GetInteractablesIF_RightWall) _array_element)))))

(fn ChangeCollisionOfInteractActors
  (params (enable :type Boolean) (actors :type Array%20of%20Actor%20Object%20References))
  (for _array_element actors
    (Collision|SetActorEnableCollision _array_element enable)))

(fn RemoveActorInterbyTag
  (params (tag :type Name))
  (for (_array_element _array_index) (Variables|Default|GetInteractablesIF_RightWall)
    (if (Utilities|Name|Equal(Name) (Utilities|Array|Get(acopy) (Variables|/Script/Engine.Actor|GetTags _array_element) 1) tag)
      (LocalVariables|SetToDestroy _array_element)
      (Utilities|Array|RemoveIndex (Variables|Default|GetInteractablesIF_RightWall) _array_index)
      (Actor|DestroyActor (LocalVariables|GetToDestroy))
      (return true)))
  (for (_array_element_2 _array_index_2) (Variables|Default|GetInteractablesBehind_RightWall)
    (if (Utilities|Name|Equal(Name) (Utilities|Array|Get(acopy) (Variables|/Script/Engine.Actor|GetTags _array_element_2) 1) tag)
      (LocalVariables|SetToDestroy _array_element_2)
      (Utilities|Array|RemoveIndex (Variables|Default|GetInteractablesBehind_RightWall) _array_index_2)
      (Actor|DestroyActor (LocalVariables|GetToDestroy))
      (return true))))

(fn ChangeCollisionbyTagInteract
  (params (Tag :type Name) (Enable :type Boolean))
  (for _array_element (Variables|Default|GetInteractablesIF_RightWall)
    (if (Utilities|Name|Equal(Name) (Utilities|Array|Get(acopy) (Variables|/Script/Engine.Actor|GetTags _array_element) 1) Tag)
      (Collision|SetActorEnableCollision _array_element Enable)))
  (for _array_element_2 (Variables|Default|GetInteractablesBehind_RightWall)
    (if (Utilities|Name|Equal(Name) (Utilities|Array|Get(acopy) (Variables|/Script/Engine.Actor|GetTags _array_element_2) 1) Tag)
      (Collision|SetActorEnableCollision _array_element_2 Enable))))