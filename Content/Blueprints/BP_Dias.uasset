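; BP_Dias is a test Blueprint for a skippable delay, with debug prints as its only output.
; BeginPlay starts two CustomDelay calls at staggered times and fires SkipPlease between them to set the Skip flag.
; CustomDelay clears Skip and runs a short fixed Delay, but its Skip check and Completed/Skipped exits are disconnected, so neither result prints.
; TimerFinished only prints placeholder text and is not called here.
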(event Custom|SkipPlease
  (Variables|Default|SetSkip true))

(event EventBeginPlay
  (Utilities|FlowControl|Sequence
    (:then_0
      (Utilities|CustomDelay 3.0
        (:Completed
          (Development|PrintString "gggg" true true "(R=0.000000,G=0.660000,B=1.000000,A=1.000000)" 44.0))
        (:Skipped
          (Development|PrintString "Skipped"))))
    (:then_1
      (Utilities|FlowControl|Delay 0.5)
      (CallFunction|SkipPlease))
    (:then_2
      (Utilities|FlowControl|Delay 1.0)
      (Utilities|CustomDelay 3.0
        (:Completed
          (Development|PrintString "kkkk" true true "(R=0.000000,G=0.660000,B=1.000000,A=1.000000)" 44.0))
        (:Skipped
          (Development|PrintString "Skipped 2"))))))

(fn ConstructionScript)

(fn TimerFinished
  (Development|PrintString "asfsa"))