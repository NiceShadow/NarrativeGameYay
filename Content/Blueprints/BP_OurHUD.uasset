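; BP_OurHUD is the game's HUD, which spawns the main on-screen widgets when play begins.
; It creates the menu, game UI and dialogue window, stores a reference to each and adds them to the viewport, giving the game UI an explicit Z-order.
; It then casts the first player controller to BP_OurPC and calls SetupRefs on it once the widgets exist.
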(event EventBeginPlay
  (Class|Actor|SetTickablewhenPaused false)
  (bind _returnvalue (UserInterface|CreateWidget "/Game/Lewin/UI/WB_Menu.WB_Menu_C"))
  (bind _output_get (Variables|Default|SetMenuRef _returnvalue))
  (UserInterface|Viewport|AddtoViewport _output_get 0)
  (bind _returnvalue_2 (UserInterface|CreateWidget "/Game/Lewin/UI/WB_GameUI.WB_GameUI_C"))
  (bind _output_get_2 (Variables|Default|SetGameUI _returnvalue_2))
  (UserInterface|Viewport|AddtoViewport _output_get_2 1)
  (bind _returnvalue_3 (UserInterface|CreateWidget "/Game/Daniel/Blueprints/BP_DialogueWindow.BP_DialogueWindow_C" (Game|GetPlayerController 0)))
  (bind _output_get_3 (Variables|Default|SetDialogueWindow _returnvalue_3))
  (UserInterface|Viewport|AddtoViewport _output_get_3 0)
  (bind _asbp_our_pc (Utilities|Casting|CastToBP_OurPC (Game|GetPlayerController 0)))
  (Default|SetupRefs _asbp_our_pc))

(fn ConstructionScript)